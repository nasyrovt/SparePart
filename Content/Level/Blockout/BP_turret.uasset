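; BP_turret is a blockout turret actor that repeatedly fires standard bullets along its right vector.
; BeginPlay waits an unsynced delay before enabling fire, letting placed turrets be offset from one another.
; Tick then runs a delay as the shot interval, spawns a bullet at the turret's location with a configurable speed, and sets its direction.
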(event `self.ReceiveBeginPlay`
  (`KismetSystemLibrary.Delay` (`self.UnsyncedWaitTime`))
  (set `self.hasWaited` true))

(event `self.ReceiveTick`
  (params (DeltaSeconds :type "Float (single-precision)"))
  (if (`self.hasWaited`)
    (`KismetSystemLibrary.Delay` (`self.TimeBetweenShoots`))
    (bind _returnvalue (`|SpawnActorFromClass` "/Game/TopDown/Equipment/BodyParts/Arms/BP_Bullet_Standard.BP_Bullet_Standard_C" (`KismetMathLibrary.Conv_VectorToTransform` (`self.K2_GetActorLocation`)) "AlwaysSpawn" "MultiplyWithRoot" null (`self.BulletSpeed`) null))
    (bind _asbp_bullet (cast `/Game/TopDown/Equipment/BodyParts/Arms/BP_Bullet` _returnvalue))
    (set `/Game/TopDown/Equipment/BodyParts/Arms/BP_Bullet.Direction` (`self.GetActorRightVector`) _asbp_bullet)))

(fn `UserConstructionScript`)